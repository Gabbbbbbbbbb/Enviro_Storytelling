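; BP_LockerDoor is an office locker door that swings open and closed.
; Open plays a timeline whose RotationMovement track sets the Door component's relative yaw, and Close reverses that same timeline.
; The ActivatedAdditives and DeactivateAdditives functions trigger Open and Close respectively.
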(event Custom|Open
  (bind _rotation_movement (Timeline|Timeline Play)
    (:Update
      (Transformation|SetRelativeRotation (Variables|Default|GetDoor) (Math|Rotator|MakeRotator 0.0 0.0 _rotation_movement) false false))))

(event Custom|Close
  (bind _rotation_movement (Timeline|Timeline Reverse)
    (:Update
      (Transformation|SetRelativeRotation (Variables|Default|GetDoor) (Math|Rotator|MakeRotator 0.0 0.0 _rotation_movement) false false))))

(event EventBeginPlay
  (|CallParentFunction) ; This node is disabled and will not be called.\nDrag off pins to build functionality.
)

(event Collision|EventActorBeginOverlap
  (params (OtherActor :type Actor%20Object%20Reference)))

(event EventTick
  (params (DeltaSeconds :type Float%20%28single-precision%29)))

(fn ConstructionScript
  (|CallParentFunction))

(fn ActivatedAdditives
  (CallFunction|Open))

(fn DeactivateAdditives
  (CallFunction|Close))