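; BP_OpenableDrawer is a drawer actor that slides open and closed when its ActivatedAdditives and DeactivateAdditives functions call Open and Close.
; Each event plays its own timeline from the start, shifting the actor one unit backward or forward along its forward vector on every update.
; Travel distance therefore depends on update count, and the start position saved in DefaultPosition at BeginPlay is never read here.
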(event Custom|Open
  (Timeline|OpenAnim PlayFromStart
    (:Update
      (Transformation|SetActorLocation (- (Transformation|GetActorLocation) (* (Transformation|GetActorForwardVector) 1.0)) false false))))

(event Custom|Close
  (Timeline|Timeline PlayFromStart
    (:Update
      (Transformation|SetActorLocation (+ (Transformation|GetActorLocation) (* (Transformation|GetActorForwardVector) 1.0)) false false))))

(event EventBeginPlay
  (|CallParentFunction)
  (Variables|Default|SetDefaultPosition (Transformation|GetActorLocation)))

(event Collision|EventActorBeginOverlap
  (params (OtherActor :type Actor%20Object%20Reference)))

(event EventTick
  (params (DeltaSeconds :type Float%20%28single-precision%29)))

(fn ConstructionScript
  (|CallParentFunction))

(fn ActivatedAdditives
  (CallFunction|Open))

(fn DeactivateAdditives
  (CallFunction|Close))