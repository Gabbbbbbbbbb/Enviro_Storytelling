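; BP_OpenableDrawerMiddle is an office drawer that slides open and closed.
; BeginPlay stores the static mesh's relative location as the closed position.
; Open eases the mesh to a Destination offset and Close eases it back, both using timed MoveComponentTo calls.
; The ActivatedAdditives and DeactivateAdditives functions trigger Open and Close respectively.
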(event Custom|Open
  (Components|MoveComponentTo (Variables|Default|GetStaticMesh) (Variables|Default|GetDestination) "0, 0, 0" true true 0.6 false))

(event Custom|Close
  (Components|MoveComponentTo (Variables|Default|GetStaticMesh) (Variables|Default|GetDefaultPosition) "0, 0, 0" true true 0.6 false))

(event EventBeginPlay
  (|CallParentFunction)
  (Variables|Default|SetDefaultPosition (Variables|/Script/Engine.SceneComponent|GetRelativeLocation (Variables|Default|GetStaticMesh))))

(event Collision|EventActorBeginOverlap
  (params (OtherActor :type Actor%20Object%20Reference)))

(event EventTick
  (params (DeltaSeconds :type Float%20%28single-precision%29)))

(fn ConstructionScript
  (|CallParentFunction))

(fn ActivatedAdditives
  (CallFunction|Open))

(fn DeactivateAdditives
  (CallFunction|Close))