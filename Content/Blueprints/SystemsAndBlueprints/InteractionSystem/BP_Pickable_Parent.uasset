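; BP_Pickable_Parent is a base pickable item in the interaction system that unlocks other interactions when taken.
; Interact sets ConditionTrue on every linked entry in InteractionsToUnlock0, spawns a pickup effect at the mesh, plays a 2D sound and destroys the actor.
; Overlap with a component tagged "Pickable" activates the NSShine effect.
; End overlap does nothing, as the shine deactivation nodes are disconnected.
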(event OnComponentBeginOverlap(StaticMesh)
  (params (OverlappedComponent :type Primitive%20Component%20Object%20Reference) (OtherActor :type Actor%20Object%20Reference) (OtherComp :type Primitive%20Component%20Object%20Reference) (OtherBodyIndex :type Integer) (bFromSweep :type Boolean) (SweepResult :type Hit%20Result%20Structure%20%28by%20ref%29))
  (if (Components|ComponentHasTag OtherComp "Pickable")
    (Components|Activation|Activate (Variables|Default|GetNS_Shine) false)))

(event OnComponentEndOverlap(StaticMesh)
  (params (OverlappedComponent :type Primitive%20Component%20Object%20Reference) (OtherActor :type Actor%20Object%20Reference) (OtherComp :type Primitive%20Component%20Object%20Reference) (OtherBodyIndex :type Integer)))

(event EventBeginPlay
  (|CallParentFunction))

(event Collision|EventActorBeginOverlap
  (params (OtherActor :type Actor%20Object%20Reference)))

(event EventTick
  (params (DeltaSeconds :type Float%20%28single-precision%29)))

(event EventInteract
  (for _array_element (Variables|Default|GetInteractionsToUnlock_0)
    (Variables|/Game/Blueprints/SystemsAndBlueprints/InteractionSystem/BP_Interactable_Parent.BP_Interactable_Parent_C|SetConditionTrue? _array_element true))
  (Niagara|SpawnSystematLocation (Variables|Default|GetVFXPickableTaken) (Transformation|GetWorldLocation (Variables|Default|GetStaticMesh)))
  (Audio|PlaySound2D (Variables|Default|GetSoundActivated) 1.0 1.0 0.0 0 0)
  (Actor|DestroyActor))

(fn ConstructionScript
  (|CallParentFunction))