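; Base interactable actor that toggles linked systems when the player character sends an interact input, optionally gated by a condition or limited to one use.
; CheckTrue and CheckFalse show or hide a can/can't-interact prompt, either as HUD widgets or the Prompt component.
; Interact flips each system's Activation/Deactivation, swaps material and sound, and calls empty additive hooks for children.
; The InteractionsToUnlock loop is disconnected and SetCurrentInteraction is empty.
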(event Custom|CheckTrue
  (bind _prompt (Variables|Default|GetPrompt))
  (bind _widgetcantinteractdata (Variables|Widgets|GetWidgetCantInteractData))
  (bind _widgetcaninteractdata (Variables|Widgets|GetWidgetCanInteractData))
  (bind _prompt_2 (Variables|Default|GetPrompt))
  ;[0.2679 1 0] Set the current interaction to itself
  (if (not (and (Variables|Booleans|GetInteractableOnce?) (Variables|Booleans|GetInteracted%20?)))
    ;[0 1 0.9293] UI Prompt activate
    (if (Variables|Booleans|GetHaveCondition?)
      (if (Variables|Booleans|GetConditionTrue?)
        (if (Variables|Widgets|GetWidgetIsOnHUD?) :!label _label
          (Utilities|IsValid _widgetcaninteractdata
            (:Is%20Valid
              (UserInterface|Viewport|AddtoViewport _widgetcaninteractdata 0)))
          (else
            (UserInterface|SetWidget _prompt_2 (Variables|Widgets|GetWidgetCanInteract))
            (Development|SetHiddeninGame _prompt_2 false false)))
        (elif (Variables|Widgets|GetWidgetIsOnHUD?)
          (Utilities|IsValid _widgetcantinteractdata
            (:Is%20Valid
              (UserInterface|Viewport|AddtoViewport _widgetcantinteractdata 0)))
          (else
            (UserInterface|SetWidget _prompt (Variables|Widgets|GetWidgetCantInteract))
            (Development|SetHiddeninGame _prompt false false))))
      (else
        (goto _label)))))

(event Custom|CheckFalse
  (bind _widgetcantinteractdata (Variables|Widgets|GetWidgetCantInteractData))
  (bind _widgetcaninteractdata (Variables|Widgets|GetWidgetCanInteractData))
  (bind _prompt (Variables|Default|GetPrompt))
  ;[0 1 0.9293] UI Prompt deactivate
  (if (Variables|Widgets|GetWidgetIsOnHUD?)
    (Utilities|FlowControl|Sequence
      (:then_0
        (Utilities|IsValid _widgetcaninteractdata
          (:Is%20Valid
            (Widget|RemovefromParent _widgetcaninteractdata))))
      (:then_1
        (Utilities|IsValid _widgetcantinteractdata
          (:Is%20Valid
            (Widget|RemovefromParent _widgetcantinteractdata)))))
    (else
      (Utilities|IsValid _prompt
        (:Is%20Valid
          (Development|SetHiddeninGame _prompt true false))))))

(event EventBeginPlay
  (bind _widgetcaninteract (Variables|Widgets|GetWidgetCanInteract))
  (bind _widgetcantinteract (Variables|Widgets|GetWidgetCantInteract))
  ;[0 1 0.9293] Set by default the material on the deactivated one
  (Rendering|Material|SetMaterial (Variables|Default|GetStaticMesh) (Variables|Material|GetMaterialToChangeIndex) (Variables|Material|GetMaterialDeactivated)) ; Material when deactivated
  ;[0 1 0.9293] UI Prompt Deactivate
  (if (Variables|Widgets|GetWidgetIsOnHUD?)
    (Utilities|IsValid _widgetcaninteract
      (:Is%20Valid
        (bind _returnvalue (UserInterface|CreateWidget (Utilities|GetClass _widgetcaninteract) (Game|GetPlayerController 0) (Variables|/Game/Blueprints/SystemsAndBlueprints/_Common_Widget/W_Can_Interact.W_Can_Interact_C|GetMake%20is%20Text _widgetcaninteract) (Variables|/Game/Blueprints/SystemsAndBlueprints/_Common_Widget/W_Can_Interact.W_Can_Interact_C|GetTo%20Do%20Text _widgetcaninteract) (Variables|/Game/Blueprints/SystemsAndBlueprints/_Common_Widget/W_Can_Interact.W_Can_Interact_C|GetImage%20Tuto _widgetcaninteract)))
        (Variables|Widgets|SetWidgetCanInteractData _returnvalue))
      (:Is%20Not%20Valid
        _))
    (Utilities|IsValid _widgetcantinteract
      (:Is%20Valid
        (bind _returnvalue_2 (UserInterface|CreateWidget (Utilities|GetClass _widgetcantinteract) (Game|GetPlayerController 0) (Variables|/Game/Blueprints/SystemsAndBlueprints/_Common_Widget/W_Cant_Interact.W_Cant_Interact_C|GetCan%20Do%20because%20? _widgetcantinteract)))
        (Variables|Widgets|SetWidgetCantInteractData _returnvalue_2)))
    (else
      (Development|SetHiddeninGame (Variables|Default|GetPrompt) true false))))

(event EventInputPressed
  ;[1 0 0] Make Interact behavior when input pressed (received from the player character)
  (CallFunction|Interact))

(fn ConstructionScript)

(fn ActivatedAdditives)

(fn DeactivateAdditives)

(fn Interact
  (bind _widgetcantinteractdata (Variables|Widgets|GetWidgetCantInteractData))
  (bind _prompt (Variables|Default|GetPrompt))
  (bind _widgetcaninteractdata (Variables|Widgets|GetWidgetCanInteractData))
  (bind _prompt_2 (Variables|Default|GetPrompt))
  (bind _staticmesh (Variables|Default|GetStaticMesh))
  ;[1 0.8626 0] For each systems linked to this interaction, activate it or deactivate it depending on the current state.
  (if (Variables|Booleans|GetHaveCondition?)
    (if (Variables|Booleans|GetConditionTrue?)
      (if (not (and (Variables|Booleans|GetInteractableOnce?) (Variables|Booleans|GetInteracted%20?))) :!label _label
        (for _array_element (Variables|Default|GetSystemsToLink)
          (if (Variables|/Game/Blueprints/SystemsAndBlueprints/InteractionSystem/BP_System_Parent.BP_System_Parent_C|GetActivated%20? _array_element)
            ;;[0 0.6366 1] Override these functions in the children of the BP_System to make specific behaviors.
            (Default|Deactivation _array_element)
            (Variables|/Game/Blueprints/SystemsAndBlueprints/InteractionSystem/BP_System_Parent.BP_System_Parent_C|SetActivated%20? _array_element false)
            (else
              (Default|Activation _array_element)
              (Variables|/Game/Blueprints/SystemsAndBlueprints/InteractionSystem/BP_System_Parent.BP_System_Parent_C|SetActivated%20? _array_element true))))
        ;[1 0.3426 0] Will set the "Interacted ?" boolean to true or false depending on the current "Interacted ?" state.
        (if (Variables|Booleans|GetInteracted%20?)
          (Variables|Booleans|SetInteracted%20? false)
          ;[1 0.3426 0] You can set the material depending of the state
          (Rendering|Material|SetMaterial _staticmesh (Variables|Material|GetMaterialToChangeIndex) (Variables|Material|GetMaterialDeactivated)) ; Material when deactivated
          ;[1 0.3426 0] You can change the sound depending of the state
          (Audio|PlaySoundatLocation (Variables|Sound|GetSoundDeactivated) (Transformation|GetActorLocation) "0, 0, 0" 1.0 1.0 0.0 0 0 0 0)
          ;[1 0.3426 0] You can add specific behaviour on your interact state !
          (CallFunction|DeactivateAdditives)
          (else
            (Variables|Booleans|SetInteracted%20? true)
            (Rendering|Material|SetMaterial _staticmesh (Variables|Material|GetMaterialToChangeIndex) (Variables|Material|GetMaterialActivated)) ; Material when activated
            (Audio|PlaySoundatLocation (Variables|Sound|GetSoundActivated) (Transformation|GetActorLocation) "0, 0, 0" 1.0 1.0 0.0 0 0 0 0) ; Sound when deactivated
            (CallFunction|ActivatedAdditives)))
        ;[1 0.3426 0] Will check and remove the prompt if interacted and interactable once
        (if (and (Variables|Booleans|GetInteracted%20?) (Variables|Booleans|GetInteractableOnce?))
          (if (Variables|Widgets|GetWidgetIsOnHUD?)
            (Utilities|FlowControl|Sequence
              (:then_0
                (Utilities|IsValid _widgetcaninteractdata
                  (:Is%20Valid
                    (Widget|RemovefromParent _widgetcaninteractdata))))
              (:then_1
                (Utilities|IsValid _widgetcantinteractdata
                  (:Is%20Valid
                    (Widget|RemovefromParent _widgetcantinteractdata)))))
            (else
              (Utilities|IsValid _prompt_2
                (:Is%20Valid
                  (Development|SetHiddeninGame _prompt_2 true false))))))
        (return)
        (elif (not (Variables|Widgets|GetWidgetIsOnHUD?))
          (Utilities|IsValid _prompt
            (:Is%20Valid
              (Development|SetHiddeninGame _prompt true false))))))
    (else
      (goto _label))))

(fn SetCurrentInteraction
  (params (CurrentInteraction :type Object%20Object%20Reference))
  (return))