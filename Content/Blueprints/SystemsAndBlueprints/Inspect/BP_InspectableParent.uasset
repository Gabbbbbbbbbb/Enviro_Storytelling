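; Base Blueprint for inspectable objects that the player can hold in front of the camera and rotate.
; Interacting while the player holds no item moves input to the object, disables its collision, attaches it to the player's item component and places it before the camera.
; Inspect input rotates it, and the interact input during inspection restores its saved transform, collision, player input and spotlight intensity.
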(event Input|EnhancedActionEvents|EnhancedInputActionIA_Interact
  (params (ActionValue :type Boolean) (ElapsedSeconds :type Float%20%28double-precision%29) (TriggeredSeconds :type Float%20%28double-precision%29) (InputAction :type Input%20Action%20Object%20Reference :default "/Game/FPS_StarterContent/FirstPerson/Input/Actions/IA_Interact.IA_Interact"))
  (bind _player_character (Variables|Default|GetPlayer%20Character))
  (:Started
    (if (Variables|/Game/_GameManager/BP_FirstPersonCharacter.BP_FirstPersonCharacter_C|GetIsInInspection? _player_character)
      (CallFunction|StopInspect)
      (Variables|/Game/_GameManager/BP_FirstPersonCharacter.BP_FirstPersonCharacter_C|SetCurrentItem _player_character 0)
      (Variables|/Game/_GameManager/BP_FirstPersonCharacter.BP_FirstPersonCharacter_C|SetIsInInspection? _player_character false))))

(event Input|EnhancedActionEvents|EnhancedInputActionIA_InspectObject
  (params (ActionValue :type Vector%202D%20Structure) (ElapsedSeconds :type Float%20%28double-precision%29) (TriggeredSeconds :type Float%20%28double-precision%29) (InputAction :type Input%20Action%20Object%20Reference :default "/Game/FPS_StarterContent/FirstPerson/Input/Actions/IA_InspectObject.IA_InspectObject"))
  (:Triggered
    (Transformation|SetActorRotation (Math|Rotator|CombineRotators (Transformation|GetActorRotation) (Math|Rotator|MakeRotator (* (.y ActionValue) 3.0) 0.0 (* (.x ActionValue) -3.0))) :!label _label))
  (:Started
    (goto _label))
  (:Ongoing
    (goto _label)))

(event EventBeginPlay
  (Variables|Default|SetBeginTransform (Transformation|GetActorTransform)))

(event EventInteractwith
  (params (PlayerCharacter :type BP%20First%20Person%20Character%20Object%20Reference))
  (bind _output_get (Variables|Default|SetPlayer%20Character PlayerCharacter))
  (Variables|/Game/_GameManager/BP_FirstPersonCharacter.BP_FirstPersonCharacter_C|GetCurrentItem _output_get
    (:then)
    (:else
      (CallFunction|StartInspect))))

(fn ConstructionScript)

(fn StartInspect
  (bind _returnvalue (Game|GetPlayerCameraManager 0))
  (bind _returnvalue_2 (Game|GetPlayerController 0))
  (bind _player_character (Variables|Default|GetPlayer%20Character))
  (Input|DisableInput _player_character _returnvalue_2)
  (Input|EnableInput _returnvalue_2)
  (Rendering|Components|Light|SetIntensity (Variables|/Game/_GameManager/BP_FirstPersonCharacter.BP_FirstPersonCharacter_C|GetSpotLight _player_character) 2e+03)
  (Transformation|AttachComponentToComponent (Variables|/Game/_GameManager/BP_FirstPersonCharacter.BP_FirstPersonCharacter_C|GetItem _player_character) "None" "SnapToTarget" "SnapToTarget" "KeepRelative" true)
  (Collision|SetCollisionEnabled (Variables|Default|GetStaticMesh) "NoCollision")
  (Variables|/Game/_GameManager/BP_FirstPersonCharacter.BP_FirstPersonCharacter_C|SetCurrentItem (Variables|Default|GetPlayer%20Character) self)
  (Transformation|SetActorLocation (+ (Camera|GetCameraLocation _returnvalue) (* (Math|Vector|GetForwardVector (Camera|GetCameraRotation _returnvalue)) (Variables|Default|GetInspectDistance))) false false))

(fn StopInspect
  (bind _returnvalue (Game|GetPlayerController 0))
  (bind _player_character (Variables|Default|GetPlayer%20Character))
  (Input|DisableInput _returnvalue)
  (Input|EnableInput _player_character _returnvalue)
  (Rendering|Components|Light|SetIntensity (Variables|/Game/_GameManager/BP_FirstPersonCharacter.BP_FirstPersonCharacter_C|GetSpotLight _player_character) 13782.667969)
  (Transformation|SetActorTransform (Variables|Default|GetBeginTransform))
  (Transformation|DetachFromActor "KeepWorld" "KeepWorld" "KeepWorld")
  (Collision|SetCollisionEnabled (Variables|Default|GetStaticMesh) "QueryAndPhysics"))