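; Parent Blueprint for interactable objects that toggle linked systems when the player uses them, optionally only once or behind a condition.
; Box overlap registers the actor with the player's AC_Interact component and shows a can or can't interact prompt.
; Input forwarded from the player runs Interact, which flips each linked system's activation and its own state, material and sound.
; Empty ActivatedAdditives and DeactivateAdditives hooks allow extra per-state behavior.
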(event OnComponentBeginOverlap(Box)
  (params (OverlappedComponent :type Primitive%20Component%20Object%20Reference) (OtherActor :type Actor%20Object%20Reference) (OtherComp :type Primitive%20Component%20Object%20Reference) (OtherBodyIndex :type Integer) (bFromSweep :type Boolean) (SweepResult :type Hit%20Result%20Structure%20%28by%20ref%29))
  (bind _prompt (Variables|Default|GetPrompt))
  (bind _prompt_2 (Variables|Default|GetPrompt))
  ;[0.2679 1 0] Set the current interaction to itself
  (if (and (== OtherActor (Game|Player|GetPlayerPawn 0)) (Utilities|DoesObjectImplementInterface OtherActor "/Game/Blueprints/InteractionSystem/BPI_Interact.BPI_Interact_C"))
    (Variables|Default|SetPlayer OtherActor)
    (if (not (and (Variables|Booleans|GetInteractableOnce?) (Variables|Booleans|GetInteracted%20?)))
      (bind _output_get (Variables|Default|SetInteractionComponent (Actor|GetComponentbyClass OtherActor "/Game/Blueprints/InteractionSystem/AC_Interact.AC_Interact_C")))
      (Default|SetCurrentInteraction _output_get self)
      ;[0 1 0.9293] UI Prompt activate
      (if (Variables|Booleans|GetHaveCondition?)
        (if (Variables|Booleans|GetConditionTrue?)
          (UserInterface|SetWidget _prompt_2 (Variables|Widgets|GetWidgetCanInteract) :!label _label)
          (Development|SetHiddeninGame _prompt_2 false false)
          (Development|PrintString "Can Interact")
          (else
            (UserInterface|SetWidget _prompt (Variables|Widgets|GetWidgetCantInteract))
            (Development|SetHiddeninGame _prompt false false)
            (Development|PrintString "Need condition !")))
        (else
          (goto _label)))
      (else
        (Development|PrintString "Already interacted")))))

(event OnComponentEndOverlap(Box)
  (params (OverlappedComponent :type Primitive%20Component%20Object%20Reference) (OtherActor :type Actor%20Object%20Reference) (OtherComp :type Primitive%20Component%20Object%20Reference) (OtherBodyIndex :type Integer))
  (bind _prompt (Variables|Default|GetPrompt))
  ;[0.2679 1 0] Reset the current Interaction to null
  (if (== OtherActor (Variables|Default|GetPlayer))
    (Default|SetCurrentInteraction (Variables|Default|GetInteractionComponent))
    ;[0 1 0.9293] UI Prompt deactivate
    (Utilities|IsValid _prompt
      (:Is%20Valid
        (Development|SetHiddeninGame _prompt true false)))))

(event EventBeginPlay
  ;[0 1 0.9293] UI Prompt Deactivate
  (Development|SetHiddeninGame (Variables|Default|GetPrompt) true false)
  ;[0 1 0.9293] Set by default the material on the deactivated one
  (Rendering|Material|SetMaterial (Variables|Default|GetStaticMesh) 0 (Variables|Material|GetMaterialDeactivated)) ; Material when deactivated
)

(event EventInputPressed
  ;[1 0 0] Make Interact behavior when input pressed (received from the player character)
  (if (Variables|Booleans|GetHaveCondition?)
    (if (Variables|Booleans|GetConditionTrue?)
      (CallFunction|Interact :!label _label)
      (Development|PrintString "Interacted"))
    (else
      (goto _label))))

(fn ConstructionScript)

(fn ActivatedAdditives)

(fn DeactivateAdditives)

(fn Interact
  (bind _prompt (Variables|Default|GetPrompt))
  (bind _staticmesh (Variables|Default|GetStaticMesh))
  ;[1 0.8626 0] For each systems linked to this interaction, activate it or deactivate it depending on the current state.
  (if (not (and (Variables|Booleans|GetInteractableOnce?) (Variables|Booleans|GetInteracted%20?)))
    (for _array_element (Variables|Default|GetSystemsToLink)
      (if (Variables|/Game/Blueprints/InteractionSystem/BP_System_Parent.BP_System_Parent_C|GetActivated%20? _array_element)
        ;;[0 0.6366 1] Override these functions in the children of the BP_System to make specific behaviors.
        (Default|Deactivation _array_element)
        (Variables|/Game/Blueprints/InteractionSystem/BP_System_Parent.BP_System_Parent_C|SetActivated%20? _array_element false)
        (else
          (Default|Activation _array_element)
          (Variables|/Game/Blueprints/InteractionSystem/BP_System_Parent.BP_System_Parent_C|SetActivated%20? _array_element true))))
    ;[1 0.3426 0] Will set the "Interacted ?" boolean to true or false depending on the current "Interacted ?" state.
    (if (Variables|Booleans|GetInteracted%20?)
      (Variables|Booleans|SetInteracted%20? false)
      ;[1 0.3426 0] You can set the material depending of the state
      (Rendering|Material|SetMaterial _staticmesh 0 (Variables|Material|GetMaterialDeactivated)) ; Material when deactivated
      ;[1 0.3426 0] You can change the sound depending of the state
      (Audio|PlaySoundatLocation (Variables|Sound|GetSoundDeactivated) (Transformation|GetActorLocation) "0, 0, 0" 1.0 1.0 0.0 0 0 0 0)
      ;[1 0.3426 0] You can add specific behaviour on your interact state !
      (CallFunction|DeactivateAdditives)
      (else
        (Variables|Booleans|SetInteracted%20? true)
        (Rendering|Material|SetMaterial _staticmesh 0 (Variables|Material|GetMaterialActivated)) ; Material when activated
        (Audio|PlaySoundatLocation (Variables|Sound|GetSoundActivated) (Transformation|GetActorLocation) "0, 0, 0" 1.0 1.0 0.0 0 0 0 0) ; Sound when deactivated
        (CallFunction|ActivatedAdditives)))
    (return)
    (else
      (Utilities|IsValid _prompt
        (:Is%20Valid
          (Development|SetHiddeninGame _prompt true false))))))

(fn SetCurrentInteraction
  (params (CurrentInteraction :type Object%20Object%20Reference))
  (return))