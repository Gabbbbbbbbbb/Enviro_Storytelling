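; Parent Blueprint for pickable objects in the interaction system, consumed when the player interacts with them.
; On Interact, it sets ConditionTrue on every entry in InteractionsToUnlock, so taking the pickup unlocks other interactions.
; It then spawns the VFXPickableTaken Niagara effect, using the static mesh's relative location as the world spawn position, and destroys itself.
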(event EventBeginPlay
  (|CallParentFunction) ; This node is disabled and will not be called.\nDrag off pins to build functionality.
)

(event Collision|EventActorBeginOverlap
  (params (OtherActor :type Actor%20Object%20Reference)))

(event EventTick
  (params (DeltaSeconds :type Float%20%28single-precision%29)))

(event EventInteract
  (for _array_element (Variables|Default|GetInteractionsToUnlock)
    (Variables|/Game/Blueprints/InteractionSystem/BP_Interactable_Parent.BP_Interactable_Parent_C|SetConditionTrue? _array_element true))
  (Niagara|SpawnSystematLocation (Variables|Default|GetVFXPickableTaken) (Variables|/Script/Engine.SceneComponent|GetRelativeLocation (Variables|Default|GetStaticMesh)))
  (Actor|DestroyActor))

(fn ConstructionScript
  (|CallParentFunction))